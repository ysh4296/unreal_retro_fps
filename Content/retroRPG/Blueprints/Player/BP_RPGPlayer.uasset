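; BP_RPGPlayer is the player character, handling movement and look input, HUD creation and an equipped weapon.
; EquipWeapon swaps the class of the Weapon child actor component, initializes it through BPI_PlayerWeapon and plays its draw sequence.
; Tick passes movement state to the weapon's shaking function.
; FireWeapon input triggers firing through the Ability System Component, activating abilities by gameplay tag.
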(event Custom|EquipWeapon
  (params (Weapon :type BP%20Player%20Weapon%20Base%20Class%20Reference))
  (bind _childactor (Variables|/Script/Engine.ChildActorComponent|GetChildActor (Variables|Default|GetWeapon)))
  (bind _output_get (Variables|Player|SetCurrentWeapon Weapon))
  (ChildActorComponent|SetChildActorClass (Variables|Default|GetWeapon) _output_get)
  (if (Utilities|DoesObjectImplementInterface _childactor "/Game/retroRPG/Blueprints/Interfaces/BPI_PlayerWeapon.BPI_PlayerWeapon_C")
    (Class|BPIPlayerWeapon|InitializeWeapon(Message) _childactor)
    (bind _asbp_player_weapon_base (Utilities|Casting|CastToBP_PlayerWeaponBase (Variables|/Script/Engine.ChildActorComponent|GetChildActor (Variables|Default|GetWeapon))))
    (Sequencer|Player|Play (Variables|/Script/ActorSequence.ActorSequenceComponent|GetSequencePlayer (Variables|/Game/retroRPG/Blueprints/Widgets/BP_PlayerWeaponBase.BP_PlayerWeaponBase_C|GetWeaponDraw _asbp_player_weapon_base)) :!class /Script/MovieScene.MovieSceneSequencePlayer)))

(event EventTick
  (params (DeltaSeconds :type Float%20%28single-precision%29))
  (bind _asbp_player_weapon_base (Utilities|Casting|CastToBP_PlayerWeaponBase (Variables|/Script/Engine.ChildActorComponent|GetChildActor (Variables|Default|GetWeapon))))
  (Default|WeaponShaking _asbp_player_weapon_base (> (Math|Vector|VectorLength (Pawn|Components|CharacterMovement|GetLastUpdateVelocity (Variables|Character|GetCharacterMovement))) 0.0) DeltaSeconds))

(event EventBeginPlay
  (bind _returnvalue (UserInterface|CreateWidget "/Game/retroRPG/Blueprints/Widgets/WBP_HUD.WBP_HUD_C"))
  (UserInterface|Viewport|AddtoViewport _returnvalue 0)
  (CallFunction|EquipWeapon "/Game/retroRPG/Blueprints/Widgets/BP_PlayerWeaponBase.BP_PlayerWeaponBase_C"))

(event Input|ActionEvents|InputActionFireWeapon
  (params (Key :type Key%20Structure :default "None"))
  ;[0.15 0.15 0.15 0.5] Default Settings with Pistol so we can always fire
  (:Pressed
    (Abilities|TryActivateAbilitiesbyTag (Variables|Default|GetAbilitySystemComponent) (Variables|Default|GetGameplayTagContainer) false)))

(event Input|AxisEvents|InputAxisHorizontalMovement
  (params (AxisValue :type Float%20%28single-precision%29))
  ;[0 0 0 0.5] Movement
  (Pawn|Input|AddMovementInput (Math|Vector|GetRightVector (Pawn|GetControlRotation :!class /Script/Engine.Pawn)) AxisValue false))

(event Input|AxisEvents|InputAxisMouseLookHorizontal
  (params (AxisValue :type Float%20%28single-precision%29))
  ;[0 0 0 0.5] FOV
  (Pawn|Input|AddControllerYawInput AxisValue))

(event Input|AxisEvents|InputAxisVerticalMovement
  (params (AxisValue :type Float%20%28single-precision%29))
  ;[0 0 0 0.5] Movement
  (Pawn|Input|AddMovementInput (Math|Vector|GetForwardVector (Pawn|GetControlRotation :!class /Script/Engine.Pawn)) AxisValue false))

(event Input|AxisEvents|InputAxisMouseLookVertical
  (params (AxisValue :type Float%20%28single-precision%29))
  ;[0 0 0 0.5] FOV
  (Pawn|Input|AddControllerPitchInput AxisValue))

(fn ConstructionScript)