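; BP_W_Pistol is the pistol weapon Blueprint for a retro RPG, driving the weapon's flipbook visuals and muzzle flash.
; InitializeWeapon shows the weapon flipbook in its idle animation.
; ShootPistol triggers a brief point-light flash and plays the fire flipbook, returning to idle after a delay equal to that flipbook's length.
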(event Custom|LightFlash
  (bind _pointlight (Variables|Default|GetPointLight))
  ;[0 0 0 0.5] Light
  (Development|SetHiddeninGame _pointlight false false)
  (Utilities|FlowControl|Delay 0.2)
  (Development|SetHiddeninGame _pointlight true false))

(event Custom|ShootPistol
  (bind _weaponflipbook (Variables|Default|GetWeaponFlipbook))
  ;[0 0 0 0.5] Set Fire Animation
  (CallFunction|LightFlash)
  (Sprite|SetFlipbook _weaponflipbook (Variables|Default|GetFireFlipbook))
  (Utilities|FlowControl|Delay (Class|PaperFlipbookComponent|GetFlipbookLength _weaponflipbook))
  (Sprite|SetFlipbook (Variables|Default|GetWeaponFlipbook) (Variables|Default|GetIdleFlipbook)))

(event EventInitializeWeapon
  ;[0 0 0 0.5] Equip Weapon
  (Sprite|SetFlipbook (Variables|Default|GetWeaponFlipbook) (Variables|Default|GetIdleFlipbook))
  (Development|SetHiddeninGame (Variables|Default|GetWeaponFlipbook) false false))

(fn ConstructionScript
  (|CallParentFunction))