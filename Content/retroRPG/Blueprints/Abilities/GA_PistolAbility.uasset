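; Pistol gameplay ability that fires the player's weapon and is meant to apply an effect to the character hit.
; FireWeapon caches the owning player and child-actor pistol, calls ShootPistol, then casts the trace result for ApplyEffect.
; GetLineTrace traces Visibility from the camera, but its end point omits the start offset.
; Its return node is unreachable, so the hit actor is never passed back.
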(event EventFireWeapon
  (bind _playerpistolweaponcomponent (Variables|Default|GetPlayerPistolWeaponComponent))
  ;[0.15 0.15 0.15 0.5] Fire Pistol
  (CallFunction|GetPlayer)
  (CallFunction|GetWeapon)
  (Utilities|IsValid _playerpistolweaponcomponent
    (:Is%20Valid
      (Default|ShootPistol _playerpistolweaponcomponent)
      (bind _actor (CallFunction|GetLineTrace))
      (bind _asretro_rpgcharactor (Utilities|Casting|CastToRetroRPGCharactor _actor))
      (CallFunction|ApplyEffect (Variables|Default|GetPlayer) _asretro_rpgcharactor))))

(fn GetPlayer
  (Utilities|IsValid (Variables|Default|GetPlayer)
    (:Is%20Valid
      _)
    (:Is%20Not%20Valid
      (bind _asbp_rpgplayer (Utilities|Casting|CastToBP_RPGPlayer (.owneractor (Ability|GetActorInfo))))
      (Variables|Default|SetPlayer _asbp_rpgplayer)))
  (return))

(fn GetWeapon
  (Utilities|IsValid (Variables|Default|GetPlayerPistolWeaponComponent)
    (:Is%20Valid
      (return))
    (:Is%20Not%20Valid
      (bind _asbp_w_pistol (Utilities|Casting|CastToBP_W_Pistol (Variables|/Script/Engine.ChildActorComponent|GetChildActor (Variables|/Game/retroRPG/Blueprints/Player/BP_RPGPlayer.BP_RPGPlayer_C|GetWeapon (Variables|Default|GetPlayer))))
        (:then
          (Variables|Default|SetPlayerPistolWeaponComponent _asbp_w_pistol)
          (return))
        (:CastFailed
          (Development|PrintString "no pistol"))))))

(fn GetLineTrace
  (bind _player (Variables|Default|GetPlayer))
  (bind _camera (Variables|/Game/retroRPG/Blueprints/Player/BP_RPGPlayer.BP_RPGPlayer_C|GetCamera _player))
  (bind _outhit (Collision|LineTraceByChannel (Transformation|GetWorldLocation _camera) (* (Math|Vector|GetForwardVector (Transformation|GetWorldRotation _camera)) (Variables|Default|GetWeaponRange)) "TraceTypeQuery1" false 0 "None"))
  (Utilities|IsValid (.HitActor (Collision|BreakHitResult _outhit))))